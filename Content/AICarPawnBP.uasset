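; AI car pawn that drives a wheeled vehicle by setting steering and throttle on its movement component.
; Tick calls the WirelessTick custom event, which feeds SteeringCalc's result into steering and the AutoThrottle variable into throttle.
; SteeringCalc holds nodes mapping the yaw difference toward a Steering target onto a normalized steering range, but they are shown as unused.
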(event Custom|WirelessTick
  (Class|WheeledVehicleMovementComponent|SetSteeringInput (Variables|Default|GetVehicleMovement) (Utilities|SteeringCalc))
  (Class|WheeledVehicleMovementComponent|SetThrottleInput (Variables|Default|GetVehicleMovement) (Variables|Default|GetAutoThrottle)))

(event EventBeginPlay)

(event Collision|EventActorBeginOverlap
  (params (OtherActor :type Actor%20Object%20Reference)))

(event EventTick
  (params (DeltaSeconds :type Float%20%28single-precision%29))
  (CallFunction|WirelessTick))

(fn ConstructionScript)